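; Player attack component for BP_Player that runs a four-step melee combo of sword montages and a kick.
; Attack input during a swing is buffered, and SwordAttackCombo either plays the next montage by AttackIndex or resets the combo.
; A looping timer sphere-traces along the blade with a hit cooldown, while a separate single trace serves the kick.
; Hits on Damageable-tagged actors apply damage, camera shake, sound and blood effects.
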(event Custom|SwordAttack
  ;[0.07819 0.07819 0.07819 0.3098] Combo Attack
  ;;[0.07819 0.07819 0.07819 0.3098] Sword Attack
  (if (Variables|Default|GetIsAttacking?)
    (Variables|Default|SetSaveAttack? true)
    (else
      (Variables|Default|SetIsAttacking? true)
      (switch int (Variables|Default|GetAttack%20Index)
        (:0
          (CallFunction|Attack1))
        (:1
          (CallFunction|Attack2))
        (:2
          (CallFunction|Attack3))
        (:3
          (CallFunction|Attack4))))))

(event Custom|SwordAttackCombo
  ;[0.07819 0.07819 0.07819 0.3098] Combo Attack
  ;;[0.07819 0.07819 0.07819 0.3098] Combo Continue
  (if (Variables|Default|GetSaveAttack?)
    (Variables|Default|SetSaveAttack? false)
    (switch int (Variables|Default|GetAttack%20Index)
      (:0
        (CallFunction|Attack1))
      (:1
        (CallFunction|Attack2))
      (:2
        (CallFunction|Attack3))
      (:3
        (CallFunction|Attack4)))
    (else
      (CallFunction|StopCombo))))

(event Custom|StartSwordTrace
  (bind _returnvalue (Utilities|Time|SetTimerbyEvent (delegate Custom|SwordTraceLoop) 0.001 true))
  (Variables|Default|SetSwordLoop _returnvalue))

(event Custom|SwordTraceLoop
  (bind (_outhit _returnvalue) (Collision|SphereTraceByChannel (Transformation|GetWorldLocation (Variables|/Game/Player/BP_Player.BP_Player_C|GetSwordTopPoint (Variables|Default|GetCharacterBP))) (Transformation|GetWorldLocation (Variables|/Game/Player/BP_Player.BP_Player_C|GetSwordBottomPoint (Variables|Default|GetCharacterBP))) 12.0 "TraceTypeQuery1" false 0 "None" true "(R=1.000000,G=0.000000,B=0.000000,A=1.000000)" "(R=0.000000,G=1.000000,B=0.000000,A=1.000000)" 0.2))
  (if _returnvalue
    (if (Actor|ActorHasTag (.HitActor (Collision|BreakHitResult _outhit)) "Damageable")
      (Utilities|FlowControl|DoOnce false :!label _label
        (:Completed
          (Game|Damage|ApplyDamage (.HitActor (Collision|BreakHitResult _outhit)) 1e+01 0 0)
          (Camera|PlayWorldCameraShake "/Game/Blueprints/BP_SwordHitHandShake.BP_SwordHitHandShake_C" (.Location (Collision|BreakHitResult _outhit)) 0.0 2e+03)
          (CallFunction|PlaySwordHitSounds)
          (Effects|SpawnEmitteratLocation "/Game/FXs/Particles/Blood/P_Blood_Splat_Cone.P_Blood_Splat_Cone" (.Location (Collision|BreakHitResult _outhit)) (Math|Rotator|MakeRotfromXY (.Normal (Collision|BreakHitResult _outhit)) (.Normal (Collision|BreakHitResult _outhit))) "1.600000,1.600000,1.600000" true "AutoRelease")
          (Utilities|FlowControl|Delay 0.5)
          (goto _label Reset))))))

(event Custom|StopCombo
  ;[0.07819 0.07819 0.07819 0.3098] Combo Attack
  ;;[0.07819 0.07819 0.07819 0.3098] Stop Combo / Attack
  (Variables|Default|SetIsAttacking? false)
  (Variables|Default|SetAttack%20Index 0))

(event Custom|Attack4
  ;[0.07819 0.07819 0.07819 0.3098] Combo Attack
  ;;[0.07819 0.07819 0.07819 0.3098] Attack4
  (Utilities|FlowControl|DoOnce false :!label _label
    (:Completed
      (Utilities|FlowControl|Delay 0.1)
      (Animation|Montage|PlayMontage (Variables|Default|GetCharacter%20Mesh) "/Game/Characters/Mannequins/Animations/SwordAttack/Attack3_Montage.Attack3_Montage"
        (:then
          (Variables|Default|SetAttack%20Index 4)
          (goto _label Reset))))))

(event Custom|Attack1
  ;[0.07819 0.07819 0.07819 0.3098] Combo Attack
  ;;[0.07819 0.07819 0.07819 0.3098] Attack1
  (Utilities|FlowControl|DoOnce false :!label _label
    (:Completed
      (Utilities|FlowControl|Delay 0.1)
      (Animation|Montage|PlayMontage (Variables|Default|GetCharacter%20Mesh) "/Game/Characters/Mannequins/Animations/SwordAttack/Attack1_Montage.Attack1_Montage"
        (:then
          (Variables|Default|SetAttack%20Index 1)
          (goto _label Reset))))))

(event Custom|StopSwordTrace
  (Utilities|Time|ClearandInvalidateTimerbyHandle (Variables|Default|GetSwordLoop)))

(event Custom|Attack2
  ;[0.07819 0.07819 0.07819 0.3098] Combo Attack
  ;;[0.07819 0.07819 0.07819 0.3098] Attack2
  (Utilities|FlowControl|DoOnce false :!label _label
    (:Completed
      (Utilities|FlowControl|Delay 0.1)
      (Animation|Montage|PlayMontage (Variables|Default|GetCharacter%20Mesh) "/Game/Characters/Mannequins/Animations/SwordAttack/Attack2_Montage.Attack2_Montage"
        (:then
          (Variables|Default|SetAttack%20Index 2)
          (goto _label Reset))))))

(event Custom|Sphere%20Trace
  (bind _characterbp (Variables|Default|GetCharacterBP))
  (bind _sphere_trace (Variables|/Game/Player/BP_Player.BP_Player_C|GetSphere%20Trace _characterbp))
  (bind _returnvalue (Transformation|GetWorldLocation _sphere_trace))
  ;[0.07819 0.07819 0.07819 0.3098] Sphere Trace (For Step/Kick)
  (bind (_outhit _returnvalue_2) (Collision|SphereTraceByChannel _returnvalue _returnvalue 25.0 "TraceTypeQuery1" false 0 "None" true "(R=1.000000,G=0.000000,B=0.000000,A=1.000000)" "(R=0.000000,G=1.000000,B=0.000000,A=1.000000)" 0.2))
  (if _returnvalue_2
    (if (Actor|ActorHasTag (.HitActor (Collision|BreakHitResult _outhit)) "Damageable")
      (Game|Damage|ApplyDamage (.HitActor (Collision|BreakHitResult _outhit)) 1e+01 0 0)
      (Camera|PlayWorldCameraShake "/Game/Blueprints/BP_SwordHitHandShake.BP_SwordHitHandShake_C" (.Location (Collision|BreakHitResult _outhit)) 0.0 2e+03)
      (CallFunction|PlaySwordHitSounds)
      (Effects|SpawnEmitteratLocation "/Game/FXs/Particles/Blood/P_Blood_Splat_Cone.P_Blood_Splat_Cone" (.Location (Collision|BreakHitResult _outhit)) (Math|Rotator|MakeRotfromXY (.Normal (Collision|BreakHitResult _outhit)) (.Normal (Collision|BreakHitResult _outhit))) "1.600000,1.600000,1.600000" true "AutoRelease"))))

(event Custom|Attack3
  ;[0.07819 0.07819 0.07819 0.3098] Combo Attack
  ;;[0.07819 0.07819 0.07819 0.3098] Attack3
  (Utilities|FlowControl|DoOnce false :!label _label
    (:Completed
      (Utilities|FlowControl|Delay 0.1)
      (Animation|Montage|PlayMontage (Variables|Default|GetCharacter%20Mesh) "/Game/Characters/Mannequins/Animations/SwordAttack/Kick_Montage.Kick_Montage"
        (:then
          (Variables|Default|SetAttack%20Index 3)
          (goto _label Reset))))))

(event Custom|Play%20Sword%20Hit%20Sounds
  ;[1 1 1] Play Sword Hit Sounds
  (Audio|PlaySoundatLocation "/Game/Audio/MS_SwordHits.MS_SwordHits" (Transformation|GetActorLocation (Components|GetOwner)) "0, 0, 0" 1.0 1.0 0.0 0 0 0 0))

(event Input|EnhancedActionEvents|EnhancedInputActionIA_Attack
  (params (ActionValue :type Boolean) (ElapsedSeconds :type Float%20%28double-precision%29) (TriggeredSeconds :type Float%20%28double-precision%29) (InputAction :type Input%20Action%20Object%20Reference :default "/Game/ThirdPerson/Input/Actions/IA_Attack.IA_Attack"))
  ;[0.07819 0.07819 0.07819 0.3098] Combo Attack
  ;;[0.07819 0.07819 0.07819 0.3098] Attack Input
  (:Started
    (if (Variables|Default|GetCanAttack?)
      (CallFunction|SwordAttack))))

(event EventBeginPlay
  (bind _asbp_player (Utilities|Casting|CastToBP_Player (Components|GetOwner)))
  (Variables|Default|SetCharacterBP _asbp_player)
  (Variables|Default|SetCharacter%20Mesh (Variables|/Script/Engine.Character|GetMesh _asbp_player)))